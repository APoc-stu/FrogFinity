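; Player actor that moves in fixed steps on Enhanced Input, tracks a score and creates the game UI on start.
; Move inputs shift a target position, which Tick feeds into MoveComponentTo on the root, with a short timer limiting step rate.
; Jump plays an ActorSequence behind its own timed cooldown, ignoring the passed direction.
; AddScore accumulates points and updates the GameUI score text.
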(event `self.ReceiveBeginPlay`
  (`self.K2_SetActorLocation` (0.0 0.0 0.0))
  (set `self.TargetPos ` (`self.K2_GetActorLocation`))
  (bind _asplayer_controller (cast `PlayerController` (`self.GetController`)))
  (bind _returnvalue (pcsubsystem `EnhancedInputLocalPlayerSubsystem` _asplayer_controller))
  (`/Engine/EditorBlueprintResources/StandardMacros.IsValid` _returnvalue
    (:`Is Valid`
      (`EnhancedInputSubsystemInterface.AddMappingContext` _returnvalue "/Game/Input/IMC_Default.IMC_Default" 0 (struct))
      (bind _returnvalue_2 (`|CreateWidget` "/Game/Blueprints/GameUI.GameUI_C" (`GameplayStatics.GetPlayerController` 0)))
      (`UserWidget.AddToViewport` _returnvalue_2 0)
      (set `self.GameUI` _returnvalue_2))))

(event `self.ReceiveTick`
  (params (DeltaSeconds :type "Float (single-precision)"))
  (`KismetSystemLibrary.MoveComponentTo` (`self.DefaultSceneRoot`) (`self.TargetPos `)))

(event `EnhancedInput|/Game/Input/IA_MoveForward`
  (params (ActionValue :type Boolean) (ElapsedSeconds :type "Float (double-precision)") (TriggeredSeconds :type "Float (double-precision)") (InputAction :type "InputAction Object Reference" :default "/Game/Input/IA_MoveForward.IA_MoveForward"))
  (:`Triggered`
    (`self.TryMove` (100.0 0.0 0.0))))

(event `EnhancedInput|/Game/Input/IA_MoveLeft`
  (params (ActionValue :type Boolean) (ElapsedSeconds :type "Float (double-precision)") (TriggeredSeconds :type "Float (double-precision)") (InputAction :type "InputAction Object Reference" :default "/Game/Input/IA_MoveLeft.IA_MoveLeft"))
  (:`Triggered`
    (`self.TryMove` (0.0 -100.0 0.0))))

(event `EnhancedInput|/Game/Input/IA_MoveRight`
  (params (ActionValue :type Boolean) (ElapsedSeconds :type "Float (double-precision)") (TriggeredSeconds :type "Float (double-precision)") (InputAction :type "InputAction Object Reference" :default "/Game/Input/IA_MoveRight.IA_MoveRight"))
  (:`Triggered`
    (`self.TryMove` (0.0 100.0 0.0))))

(event `EnhancedInput|/Game/Input/IA_MoveBack`
  (params (ActionValue :type Boolean) (ElapsedSeconds :type "Float (double-precision)") (TriggeredSeconds :type "Float (double-precision)") (InputAction :type "InputAction Object Reference" :default "/Game/Input/IA_MoveBack.IA_MoveBack"))
  (:`Triggered`
    (`self.TryMove` (-100.0 0.0 0.0))))

(event `EnhancedInput|/Game/Input/IA_Jump`
  (params (ActionValue :type Boolean) (ElapsedSeconds :type "Float (double-precision)") (TriggeredSeconds :type "Float (double-precision)") (InputAction :type "InputAction Object Reference" :default "/Game/Input/IA_Jump.IA_Jump"))
  (:`Triggered`
    (`self.TryJump` (0.0 0.0 100.0))))

(fn `AddScore`
  (params (ScoreToAdd :type Integer))
  (bind _output_get (set `self.Score ` (+ ScoreToAdd (`self.Score `))))
  (`/Game/Blueprints/GameUI.UpdateScoreText` (`self.GameUI`) _output_get))

(fn `EnableCanMove`
  (set `self.CanMove ` true))

(fn `TryJump`
  (params (Direction :type "Vector Structure"))
  (if (`self.Canjump`)
    (`ActorSequenceComponent.PlaySequence` (`self.ActorSequence`))
    (set `self.Canjump` false)
    (`KismetSystemLibrary.K2_SetTimer` null "Unjump" 2.0)))

(fn `TryMove`
  (params (Direction :type "Vector Structure"))
  (if (`self.CanMove `)
    (set `self.TargetPos ` (+ Direction (`self.TargetPos `)))
    (set `self.CanMove ` false)
    (`KismetSystemLibrary.K2_SetTimer` null "EnableCanMove" 0.3)))

(fn `Unjump`
  (set `self.Canjump` true))

(fn `UserConstructionScript`)