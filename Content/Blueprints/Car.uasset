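; Car is a moving hazard actor that restarts the level when it touches the Player.
; Each tick it moves along the root component's forward vector at Speed, scaled by delta time and without sweeping.
; Once it is farther than Distance from StartPosition, it snaps back there to loop its path.
; An overlap with a Player reopens the current level by name.
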(event `self.ReceiveTick`
  (params (DeltaSeconds :type "Float (single-precision)"))
  (`self.K2_AddActorWorldOffset` (* (`SceneComponent.GetForwardVector` (`self.DefaultSceneRoot`)) (* DeltaSeconds (`self.Speed `))))
  (if (> (`KismetMathLibrary.Vector_Distance` (`self.K2_GetActorLocation`) (`self.StartPosition `)) (`self.Distance `))
    (`self.K2_SetActorLocation` (`self.StartPosition `))))

(event `self.ReceiveActorBeginOverlap`
  (params (OtherActor :type "Actor Object Reference"))
  (cast `/Game/Blueprints/Player` OtherActor)
  (bind _returnvalue (`GameplayStatics.GetCurrentLevelName` true))
  (`GameplayStatics.OpenLevel` (`KismetStringLibrary.Conv_StringToName` _returnvalue)))

(fn `UserConstructionScript`)